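; Player-drivable tank pawn that wires mesh components and input to C++ aiming and movement components.
; BeginPlay hands barrel and turret to TankAim and both tracks to TankNavMovement, while the construction script assigns their static meshes.
; Input rotates the camera gimbal and spring arm, drives forward and turn movement through TankNavMovement, and fires through TankAim.
; Per-track axis inputs are empty test stubs, with their driving-force calls left disconnected.
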(event EventBeginPlay
  ;[1 1 1] Setting Tank Components Based on C++ Code
  (Class|TankAimComponent|Initialise (Variables|Default|GetTankAim) (Variables|Default|GetTankBarrelC) (Variables|Default|GetTankTurretC))
  (Class|TankNavMovementComponent|Initialise (Variables|Default|GetTankNavMovement) (Variables|Default|GetTankTrackL) (Variables|Default|GetTankTrackR)))

(event Input|ActionEvents|InputActionFire
  (params (Key :type Key%20Structure))
  ;[1 1 1] Player Aim and Shoot Controls Binding
  (:Pressed
    (Class|TankAimComponent|FireProjectile (Variables|Default|GetTankAim))))

(event Input|AxisEvents|InputAxisAimHorizontal
  (params (AxisValue :type Float%20%28single-precision%29))
  ;[1 1 1] Player Aim and Shoot Controls Binding
  (Transformation|AddLocalRotation (Variables|Default|GetHorizontalGimbalP) (Math|Rotator|MakeRotator 0.0 0.0 AxisValue) false false))

(event Input|AxisEvents|InputAxisAimVertical
  (params (AxisValue :type Float%20%28single-precision%29))
  ;[1 1 1] Player Aim and Shoot Controls Binding
  (Transformation|AddLocalRotation (Variables|Default|GetSpringArmP) (Math|Rotator|MakeRotator 0.0 AxisValue 0.0) false false))

(event Input|AxisEvents|InputAxisTankTrackRMovement
  (params (AxisValue :type Float%20%28single-precision%29))
  ;[1 1 1] Testing (Not running)
)

(event Input|AxisEvents|InputAxisTankTrackLMovement
  (params (AxisValue :type Float%20%28single-precision%29))
  ;[1 1 1] Testing (Not running)
)

(event Input|AxisEvents|InputAxisMoveForward
  (params (AxisValue :type Float%20%28single-precision%29))
  ;[1 1 1] Player Movement Controls Bindings
  (Class|TankNavMovementComponent|MoveForward (Variables|Default|GetTankNavMovement) AxisValue))

(event Input|AxisEvents|InputAxisTurn
  (params (AxisValue :type Float%20%28single-precision%29))
  ;[1 1 1] Player Movement Controls Bindings
  (Class|TankNavMovementComponent|MoveRight (Variables|Default|GetTankNavMovement) AxisValue))

(fn ConstructionScript
  (Components|StaticMesh|SetStaticMesh (Variables|Default|GetTankTurretC) "/Game/Tank/tankTurret.tankTurret")
  (Components|StaticMesh|SetStaticMesh (Variables|Default|GetTankBarrelC) "/Game/Tank/tankBarrel.tankBarrel")
  (Components|StaticMesh|SetStaticMesh (Variables|Default|GetTankTrackR) "/Game/Tank/tankTrack.tankTrack")
  (Components|StaticMesh|SetStaticMesh (Variables|Default|GetTankTrackL) "/Game/Tank/tankTrack.tankTrack"))